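; Modular-body ghost of the player character, apparently for ghost trails, that sets itself up on BeginPlay.
; SetPose swaps hand meshes from CustomizationData rows, slaves body-part meshes to the main Mesh via Master Pose and collects the parts.
; GhostTrails gives those parts dynamic material instances and stores them; no fade or update logic is present.
; The player reference is only cached, and the pose-copy call is unconnected.
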(event Custom|GhostTrails
  (for _array_element (Variables|Default|GetbodyParts)
    (bind _returnvalue (Rendering|Material|CreateDynamicMaterialInstance (Rendering|Material|GetMaterial _array_element 0) 0 :!class /Script/Engine.KismetMaterialLibrary))
    (Utilities|Array|Add (Variables|Default|GetdynamicMats) _returnvalue)
    (Rendering|Material|SetMaterial _array_element 0 _returnvalue)))

(event EventBeginPlay
  (bind _asac_character (Utilities|Casting|CastToAC_Character (Game|Player|GetPlayerPawn 0)))
  (Variables|Default|SetPlayer _asac_character)
  (CallFunction|SetPose)
  (CallFunction|GhostTrails))

(fn ConstructionScript)

(fn SetPose
  (bind _llleg (Variables|Default|GetlLLeg))
  (bind _neck (Variables|Default|Getneck))
  (bind _chest (Variables|Default|Getchest))
  (bind _hips (Variables|Default|Gethips))
  (bind _mesh (Variables|Character|GetMesh))
  (bind _urarm (Variables|Default|GetuRArm))
  (bind _ularm (Variables|Default|GetuLArm))
  (bind _lrarm (Variables|Default|GetlRArm))
  (bind _llarm (Variables|Default|GetlLArm))
  (bind _rhand (Variables|Default|GetrHand))
  (bind _lhand (Variables|Default|GetlHand))
  (bind _urleg (Variables|Default|GetuRLeg))
  (bind _ulleg (Variables|Default|GetuLLeg))
  (bind _lrleg (Variables|Default|GetlRLeg))
  (bind _rfoot (Variables|Default|GetrFoot))
  (bind _lfoot (Variables|Default|GetlFoot))
  (for _array_element (Variables|Default|GetcustomizationList)
    (bind _returnvalue (Utilities|GetDataTableRow "/Game/airCombo/customizationData.customizationData" (Utilities|String|StringToName (Utilities|String|ToString(Integer) _array_element)))
      (:then
        (switch Utilities|FlowControl|Switch|SwitchoncustomizeSlots (.itemSlot (Utilities|Struct|BreakcustomizationStruct _returnvalue))
          (:NewEnumerator10
            (Class|SkinnedMeshComponent|SetSkeletalMesh (Variables|Default|GetlHand) (.itemModel (Utilities|Struct|BreakcustomizationStruct _returnvalue)) true))
          (:NewEnumerator14
            (Class|SkinnedMeshComponent|SetSkeletalMesh (Variables|Default|GetrHand) (.itemModel (Utilities|Struct|BreakcustomizationStruct _returnvalue)) true))))))
  (Class|SkinnedMeshComponent|SetMasterPoseComponent _neck _mesh)
  (Class|SkinnedMeshComponent|SetMasterPoseComponent _chest _mesh)
  (Class|SkinnedMeshComponent|SetMasterPoseComponent _hips _mesh)
  (Class|SkinnedMeshComponent|SetMasterPoseComponent _urarm _mesh)
  (Class|SkinnedMeshComponent|SetMasterPoseComponent _ularm _mesh)
  (Class|SkinnedMeshComponent|SetMasterPoseComponent _lrarm _mesh)
  (Class|SkinnedMeshComponent|SetMasterPoseComponent _llarm _mesh)
  (Class|SkinnedMeshComponent|SetMasterPoseComponent _rhand _mesh)
  (Class|SkinnedMeshComponent|SetMasterPoseComponent _lhand _mesh)
  (Class|SkinnedMeshComponent|SetMasterPoseComponent _urleg _mesh)
  (Class|SkinnedMeshComponent|SetMasterPoseComponent _ulleg _mesh)
  (Class|SkinnedMeshComponent|SetMasterPoseComponent _lrleg _mesh)
  (Class|SkinnedMeshComponent|SetMasterPoseComponent _llleg _mesh)
  (Class|SkinnedMeshComponent|SetMasterPoseComponent _rfoot _mesh)
  (Class|SkinnedMeshComponent|SetMasterPoseComponent _lfoot _mesh)
  (Variables|Default|SetbodyParts (Utilities|Array|MakeArray _mesh _neck _chest (Variables|Default|Gethair) _urarm _ularm _lrarm _llarm _rhand _lhand _urleg _ulleg _llleg _rfoot _lfoot _hips _lrleg 0 0)))