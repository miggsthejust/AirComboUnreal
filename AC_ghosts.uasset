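; Ghost afterimage actor that freezes a copy of the player's modular character pose in a ghost material, then destroys itself after GhostLength.
; On BeginPlay, SetPose slaves the body-part meshes to Head via master pose and looks up customization rows, though its mesh-swap nodes are disconnected.
; GhostTrails gives each part a dynamic ghost material and copies the player's mesh pose onto Head, which drives the other parts.
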(event Custom|GhostTrails
  (for _array_element (Variables|Default|GetbodyParts)
    (bind _returnvalue (Rendering|Material|CreateDynamicMaterialInstance (Rendering|Material|GetMaterial _array_element 0) "/Game/airCombo/mats/ghostMat_Inst.ghostMat_Inst" :!class /Script/Engine.KismetMaterialLibrary))
    (Utilities|Array|Add (Variables|Default|GetdynamicMats) _returnvalue)
    (Rendering|Material|SetMaterial _array_element 0 _returnvalue)
    (Class|PoseableMeshComponent|CopyPosefromSkeletalComponent (Variables|Default|Gethead) (Variables|/Script/Engine.Character|GetMesh (Variables|Default|GetPlayer)))
    (Utilities|FlowControl|Delay (Variables|Default|GetghostLength))
    (Actor|DestroyActor)))

(event EventBeginPlay
  (bind _asac_character (Utilities|Casting|CastToAC_Character (Game|Player|GetPlayerPawn 0)))
  (Variables|Default|SetPlayer _asac_character)
  (CallFunction|SetPose)
  (CallFunction|GhostTrails))

(fn ConstructionScript)

(fn SetPose
  (bind _head (Variables|Default|Gethead))
  (bind _hair (Variables|Default|Gethair))
  (for _array_element (Variables|Default|GetcustomizationList)
    (bind _returnvalue (Utilities|GetDataTableRow "/Game/airCombo/customizationData.customizationData" (Utilities|String|StringToName (Utilities|String|ToString(Integer) _array_element)))
      (:then
        (switch Utilities|FlowControl|Switch|SwitchoncustomizeSlots (.itemSlot (Utilities|Struct|BreakcustomizationStruct _returnvalue))))))
  (Class|SkinnedMeshComponent|SetMasterPoseComponent _hair _head)
  (Variables|Default|SetbodyParts (Utilities|Array|MakeArray _hair (Variables|Default|Getneck) (Variables|Default|Getchest) (Variables|Default|Gethips) (Variables|Default|GetshoulderL) (Variables|Default|GetshoulderR) (Variables|Default|GetuArmL) (Variables|Default|GetlArmL) (Variables|Default|GethandL) (Variables|Default|GetuArmR) (Variables|Default|GetlArmR) (Variables|Default|GethandR) (Variables|Default|GetuLegL) (Variables|Default|GetlLegL) (Variables|Default|GetfootL) (Variables|Default|GetuLegR) (Variables|Default|GetlLegR) (Variables|Default|GetfootR) _head)))